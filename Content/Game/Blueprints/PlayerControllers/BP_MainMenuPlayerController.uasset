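; Player controller for the main menu that shows the menu widget and handles switching to and from the settings screen.
; On BeginPlay it swaps the gameplay input mapping for the menu one, pauses the game, creates the menu widget, and enables Game and UI input with a visible cursor.
; RouteToSettings and BackfromSettings remove the current widget from its parent and construct a fresh settings or main menu widget each time.
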(event `self.ReceiveBeginPlay`
  (bind _returnvalue (subsystem `EnhancedInputLocalPlayerSubsystem`))
  (`parent.ReceiveBeginPlay`)
  (`EnhancedInputSubsystemInterface.RemoveMappingContext` _returnvalue "/Game/Game/Input/IMC_InputMapping.IMC_InputMapping" (struct))
  (`EnhancedInputSubsystemInterface.AddMappingContext` _returnvalue "/Game/Game/Input/IMC_MainMenu.IMC_MainMenu" 0 (struct))
  (`GameplayStatics.SetGamePaused` true)
  (bind _returnvalue_2 (`|GenericCreateObject` "/Game/Game/UI/BP_MainMenu.BP_MainMenu_C"))
  (bind _output_get (set `self.MainMenuWidget` _returnvalue_2))
  (`UserWidget.AddToViewport` _output_get 0)
  (`WidgetBlueprintLibrary.SetInputMode_GameAndUIEx` self _returnvalue_2 "DoNotLock" true true)
  (set `self.bShowMouseCursor` true))

(event `RouteToSettings`
  (`Widget.RemoveFromParent` (`self.MainMenuWidget`))
  (bind _returnvalue (`|GenericCreateObject` "/Game/Game/UI/Settings/BP_Settings.BP_Settings_C"))
  (bind _output_get (set `self.SettingsWidget` _returnvalue))
  (`UserWidget.AddToViewport` _output_get 0))

(event `/Game/Game/Blueprints/PlayerControllers/BP_PlayerControllerInterface.BackFromSettings`
  (`Widget.RemoveFromParent` (`self.SettingsWidget`))
  (bind _returnvalue (`|GenericCreateObject` "/Game/Game/UI/BP_MainMenu.BP_MainMenu_C"))
  (bind _output_get (set `self.MainMenuWidget` _returnvalue))
  (`UserWidget.AddToViewport` _output_get 0))

(fn `UserConstructionScript`
  (`parent.UserConstructionScript`))