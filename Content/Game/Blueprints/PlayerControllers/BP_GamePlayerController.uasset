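; Player controller for a target-shooting game, handling input, aiming, scoring and UI flow.
; It opens a start cooldown widget, then swaps to in-game and game-over screens on GameState phase changes, and routes settings back to pause or game-over menus.
; Shooting line-traces from the view point, resets hit target spheres and writes score and hit accuracy to the GameState.
; Camera look scales by GameInstance sensitivity, and the pause input toggles the pause menu.
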(event Custom|SetUI
  (switch Utilities|FlowControl|Switch|SwitchonE_GamePhase (Variables|/Game/Game/Blueprints/BP_GameState.BP_GameState_C|GetgameState (stale EventBeginPlay _asbp_game_state))
    (:NewEnumerator1
      (Widget|RemovefromParent (Variables|Default|GetStartCooldownWidget))
      (|DisplayInGame))
    (:NewEnumerator2
      (Widget|RemovefromParent (Variables|Default|GetInGameWidget))
      (|DisplayGameOver))))

(event Custom|RouteToSettings
  (params (ClosingWidget :type Widget%20Object%20Reference))
  (Widget|RemovefromParent ClosingWidget)
  (bind _returnvalue (Game|ConstructObjectfromClass "/Game/Game/UI/Settings/BP_Settings.BP_Settings_C"))
  (bind _output_get (Variables|Default|SetSettingsWidget _returnvalue))
  (UserInterface|Viewport|AddtoViewport _output_get 0))

(event EventBeginPlay
  (bind _returnvalue (PlayerController|LocalPlayerSubsystems|GetEnhancedInputLocalPlayerSubsystem))
  (Input|RemoveMappingContext _returnvalue "/Game/Game/Input/IMC_MainMenu.IMC_MainMenu" "(bIgnoreAllPressedKeysUntilRelease=True,bForceImmediately=False,bNotifyUserSettings=False)")
  (Input|AddMappingContext _returnvalue "/Game/Game/Input/IMC_InputMapping.IMC_InputMapping" 0 "(bIgnoreAllPressedKeysUntilRelease=True,bForceImmediately=False,bNotifyUserSettings=False)")
  (bind _returnvalue_2 (Game|ConstructObjectfromClass "/Game/Game/UI/GameWidgets/BP_StartCooldown.BP_StartCooldown_C"))
  (bind _output_get (Variables|Default|SetStartCooldownWidget _returnvalue_2))
  (UserInterface|Viewport|AddtoViewport _output_get 0)
  (Input|SetInputModeUIOnly self (Variables|Default|GetStartCooldownWidget) "DoNotLock" false)
  (bind _asbp_game_state (Utilities|Casting|CastToBP_GameState (Game|GetGameState)))
  (EventDispatchers|BindEventtoOnChangeGamePhase _asbp_game_state (delegate Custom|SetUI)))

(event EventBackfromSettings
  (Widget|RemovefromParent (Variables|Default|GetSettingsWidget))
  (bind _asbp_game_state (Utilities|Casting|CastToBP_GameState (Game|GetGameState))) ; If it fails, we will be in main menu
  (if (Variables|/Game/Game/Blueprints/BP_GameState.BP_GameState_C|GetgamePaused _asbp_game_state)
    (bind _asbp_game_player_controller (Utilities|Casting|CastToBP_GamePlayerController (Game|GetPlayerController 0)))
    (bind _returnvalue (Game|ConstructObjectfromClass "/Game/Game/UI/GameWidgets/BP_PauseGame.BP_PauseGame_C"))
    (bind _output_get (Variables|BP_GamePlayerController_C|SetPauseGameWidget _asbp_game_player_controller _returnvalue))
    (UserInterface|Viewport|AddtoViewport _output_get 0)
    (else
      (switch Utilities|FlowControl|Switch|SwitchonE_GamePhase (Variables|/Game/Game/Blueprints/BP_GameState.BP_GameState_C|GetgameState _asbp_game_state) ; If we are in the phase game over
        (:NewEnumerator2
          (bind _returnvalue_2 (Game|ConstructObjectfromClass "/Game/Game/UI/GameWidgets/BP_GameOver.BP_GameOver_C"))
          (bind _output_get_2 (Variables|Default|SetGameOverWidget _returnvalue_2))
          (UserInterface|Viewport|AddtoViewport _output_get_2 0))))))

(event Input|EnhancedActionEvents|EnhancedInputActionIA_CameraRotation
  (params (ActionValue :type Vector%202D%20Structure) (ElapsedSeconds :type Float%20%28double-precision%29) (TriggeredSeconds :type Float%20%28double-precision%29) (InputAction :type Input%20Action%20Object%20Reference :default "/Game/Game/Input/Actions/IA_CameraRotation.IA_CameraRotation"))
  ;[0.15 0.15 0.15 0.5] Handle camera rotation
  (bind _asbp_game_instance (Utilities|Casting|CastToBP_GameInstance (Game|GetGameInstance)))
  (Class|PlayerController|AddYawInput (* (.x ActionValue) (Variables|/Game/Game/Blueprints/BP_GameInstance.BP_GameInstance_C|Getsensitivity _asbp_game_instance)))
  (Class|PlayerController|AddPitchInput (* (Variables|/Game/Game/Blueprints/BP_GameInstance.BP_GameInstance_C|Getsensitivity _asbp_game_instance) (.y ActionValue))))

(event Input|EnhancedActionEvents|EnhancedInputActionIA_Shoot
  (params (ActionValue :type Boolean) (ElapsedSeconds :type Float%20%28double-precision%29) (TriggeredSeconds :type Float%20%28double-precision%29) (InputAction :type Input%20Action%20Object%20Reference :default "/Game/Game/Input/Actions/IA_Shoot.IA_Shoot"))
  (bind (_location _rotation) (Pawn|GetPlayerViewPoint))
  ;[0.15 0.15 0.15 0.5] Check if a target is hit by the player
  (:Started
    (bind (_outhit _returnvalue) (Collision|LineTraceByChannel _location (+ _location (* (Math|Vector|GetForwardVector _rotation) 1.5e+03)) "TraceTypeQuery1" false 0 "ForOneFrame"))
    (Utilities|FlowControl|Sequence
      (:then_0
        ;[0.15 0.15 0.15 0.5] Handle hit (Destroy target and increase score)
        (if _returnvalue
          (bind _asbp_target_sphere (Utilities|Casting|CastToBP_TargetSphere (.HitActor (Collision|BreakHitResult _outhit))))
          (Default|ResettheTarget _asbp_target_sphere)
          (bind _asbp_game_state (Utilities|Casting|CastToBP_GameState (Game|GetGameState)))
          (Variables|/Game/Game/Blueprints/BP_GameState.BP_GameState_C|Setscore _asbp_game_state (+ (Variables|/Game/Game/Blueprints/BP_GameState.BP_GameState_C|Getscore _asbp_game_state) 100))))
      (:then_1
        ;[0.15 0.15 0.15 0.5] Update variables to calculate hit accuracy(allShots stores count of all shots, hitShots only stores accurate shots)
        (if _returnvalue
          (Utilities|Casting|CastToBP_TargetSphere (.HitActor (Collision|BreakHitResult _outhit)))
          (Variables|Default|SethitShots (+ (Variables|Default|GethitShots) 1))))
      (:then_2
        (Variables|Default|SetAllShots (+ (Variables|Default|GetAllShots) 1)))
      (:then_3
        ;[0.15 0.15 0.15 0.5] Calculate hit accuracy
        (bind _asbp_game_state_2 (Utilities|Casting|CastToBP_GameState (Game|GetGameState)))
        (Variables|/Game/Game/Blueprints/BP_GameState.BP_GameState_C|Setaccuracy _asbp_game_state_2 (* (/ (Math|Conversions|ToFloat(Integer) (Variables|Default|GethitShots)) (Math|Conversions|ToFloat(Integer) (Variables|Default|GetAllShots))) 1e+02)) ; Accuracy equals hit / all * 100
      ))))

(event Input|EnhancedActionEvents|EnhancedInputActionIA_PauseGame
  (params (ActionValue :type Boolean) (ElapsedSeconds :type Float%20%28double-precision%29) (TriggeredSeconds :type Float%20%28double-precision%29) (InputAction :type Input%20Action%20Object%20Reference :default "/Game/Game/Input/Actions/IA_PauseGame.IA_PauseGame"))
  (bind _asbp_game_state (Utilities|Casting|CastToBP_GameState (Game|GetGameState)))
  (if (not (Variables|/Game/Game/Blueprints/BP_GameState.BP_GameState_C|GetgamePaused _asbp_game_state))
    ;[0.15 0.15 0.15 0.5] Pause Game
    (bind _returnvalue (Game|ConstructObjectfromClass "/Game/Game/UI/GameWidgets/BP_PauseGame.BP_PauseGame_C"))
    (bind _output_get (Variables|Default|SetPauseGameWidget _returnvalue))
    (UserInterface|Viewport|AddtoViewport _output_get 0)
    (Input|SetInputModeGameandUI self (Variables|Default|GetPauseGameWidget) "DoNotLock" true true)
    (Variables|Default|SetbShowMouseCursor true)
    (Variables|/Game/Game/Blueprints/BP_GameState.BP_GameState_C|SetgamePaused _asbp_game_state true)
    (Game|SetGamePaused true)
    (else
      ;[0.15 0.15 0.15 0.5] Resume Game
      (if (UserInterface|Viewport|IsinViewport (Variables|Default|GetPauseGameWidget))
        (Widget|RemovefromParent (Variables|Default|GetPauseGameWidget))
        (Input|SetInputModeGameOnly self true)
        (Variables|/Game/Game/Blueprints/BP_GameState.BP_GameState_C|SetgamePaused _asbp_game_state false)
        (Game|SetGamePaused false)
        (Variables|Default|SetbShowMouseCursor false)))))

(event Input|KeyboardEvents|DebugKeyQ
  (params (Key :type Key%20Structure :default "None") (ActionValue :type Input%20Action%20Value%20Structure))
  (:Pressed
    (bind _asbp_game_state (Utilities|Casting|CastToBP_GameState (Game|GetGameState)))
    (if (not (Variables|/Game/Game/Blueprints/BP_GameState.BP_GameState_C|GetgamePaused _asbp_game_state))
      ;[0.15 0.15 0.15 0.5] Pause Game
      (bind _returnvalue (Game|ConstructObjectfromClass "/Game/Game/UI/GameWidgets/BP_PauseGame.BP_PauseGame_C"))
      (bind _output_get (Variables|Default|SetPauseGameWidget _returnvalue))
      (UserInterface|Viewport|AddtoViewport _output_get 0)
      (Input|SetInputModeGameandUI self (Variables|Default|GetPauseGameWidget) "DoNotLock" true true)
      (Variables|Default|SetbShowMouseCursor true)
      (Variables|/Game/Game/Blueprints/BP_GameState.BP_GameState_C|SetgamePaused _asbp_game_state true)
      (Game|SetGamePaused true)
      (else
        ;[0.15 0.15 0.15 0.5] Resume Game
        (if (UserInterface|Viewport|IsinViewport (Variables|Default|GetPauseGameWidget))
          (Widget|RemovefromParent (Variables|Default|GetPauseGameWidget))
          (Input|SetInputModeGameOnly self true)
          (Variables|/Game/Game/Blueprints/BP_GameState.BP_GameState_C|SetgamePaused _asbp_game_state false)
          (Game|SetGamePaused false)
          (Variables|Default|SetbShowMouseCursor false))))))

(fn ConstructionScript
  (|CallParentFunction))