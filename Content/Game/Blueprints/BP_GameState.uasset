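; BP_GameState drives the round's phases from a start cooldown through timed play to game over, and resets Score and Accuracy at BeginPlay.
; Both timer start values come from BP_GameInstance, with a second added to the cooldown for a better player experience.
; Tick counts down the active phase's timer unless the game is paused, then advances GameState and fires OnChangeGamePhase at each transition.
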(event `self.ReceiveBeginPlay`
  (set `self.accuracy` 0.0)
  (set `self.score` 0)
  (bind _asbp_game_instance (cast `/Game/Game/Blueprints/BP_GameInstance` (`GameplayStatics.GetGameInstance`)))
  (set `self.startCooldown` (+ (`/Game/Game/Blueprints/BP_GameInstance.cooldownStartValue` _asbp_game_instance) 1.0))
  (set `self.gameCountdown` (`/Game/Game/Blueprints/BP_GameInstance.timerStartValue` _asbp_game_instance))
  (set `self.gameState` "NewEnumerator0"))

(event `self.ReceiveTick`
  (params (DeltaSeconds :type "Float (single-precision)"))
  (if (not (`self.gamePaused`))
    (switch `/Game/Game/Blueprints/Enums/E_GamePhase` (`self.gameState`)
      (:`NewEnumerator0`
        (bind _output_get (set `self.startCooldown` (- (`self.startCooldown`) DeltaSeconds)))
        (if (<= _output_get 1.0)
          (set `self.gameState` "NewEnumerator1")
          (`self.OnChangeGamePhase`)))
      (:`NewEnumerator1`
        (bind _output_get_2 (set `self.gameCountdown` (- (`self.gameCountdown`) DeltaSeconds)))
        (if (<= _output_get_2 0.0)
          (set `self.gameState` "NewEnumerator2")
          (`self.OnChangeGamePhase`))))))

(fn `UserConstructionScript`)