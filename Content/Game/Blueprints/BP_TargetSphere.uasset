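; BP_TargetSphere is a target that jumps to a random free spot on a three-by-three grid when reset.
; ResetTheTarget keeps the actor's X and rerolls grid Y and Z until the position is absent from the TargetLocations array on BP_GamemodeBase.
; It then removes the sphere's old location from that shared array, teleports and registers the new one, preventing overlap between targets.
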(fn `ResetTheTarget`
  (bind _returnvalue_x (`KismetMathLibrary.BreakVector` (`self.K2_GetActorLocation`)))
  (bind _asbp_gamemode_base (cast `/Game/Game/Blueprints/BP_GamemodeBase` (`GameplayStatics.GetGameMode`)))
  ; Changes the location of the target (yeah i know what you are thinking about) I added a checking to prevent overlap on targets
  (bind _returnvalue (`KismetMathLibrary.MakeVector` _returnvalue_x (`KismetMathLibrary.Conv_IntToDouble` (- (* (+ (`KismetMathLibrary.RandomInteger` 3) 1) 120) 180)) (`KismetMathLibrary.Conv_IntToDouble` (+ (* (+ (`KismetMathLibrary.RandomInteger` 3) 1) 120) 80)) :!label _label))
  (bind _targetlocations (`/Game/Game/Blueprints/BP_GamemodeBase.TargetLocations` _asbp_gamemode_base))
  (if (!= (`KismetArrayLibrary.Array_Find` _targetlocations _returnvalue) -1)
    (goto _label)
    (else
      (`KismetArrayLibrary.Array_RemoveItem` _targetlocations (`SceneComponent.K2_GetComponentLocation` (`self.Sphere`))) ; We are removing the old location
      (`self.K2_SetActorLocation` _returnvalue false true)
      (`KismetArrayLibrary.Array_Add` _targetlocations _returnvalue) ; We are storing the new location
    )))

(fn `UserConstructionScript`)